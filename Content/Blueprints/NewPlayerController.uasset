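; Player controller that opens a variable-entry widget at start and handles wall-building input.
; On BeginPlay it shows the EnterVariables widget with the mouse cursor and Game and UI input mode.
; BuildWall works only once through a DoOnce, spawning a Wall at the player character's location and opening a focused WallWidget.
; DestroyWall calls DestroyActor on the controller itself, not on the spawned Wall.
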(event EventBeginPlay
  (bind _returnvalue (UserInterface|CreateWidget "/Game/EnterVariables.EnterVariables_C" (Game|GetPlayerController 0)))
  (UserInterface|Viewport|AddtoViewport _returnvalue 0)
  (Input|SetInputModeGameandUI self _returnvalue "DoNotLock" true)
  (Variables|Default|SetbShowMouseCursor true))

(event Input|ActionEvents|InputActionBuildWall
  (params (Key :type Key%20Structure :default "None"))
  (:Pressed
    (Utilities|FlowControl|DoOnce false
      (:Completed
        (Game|SpawnActorfromClass "/Game/Wall.Wall_C" (Math|Conversions|ToTransform(Vector) (Transformation|GetActorLocation (Game|GetPlayerCharacter 0))) "Undefined" 0 0)
        (bind _returnvalue (UserInterface|CreateWidget "/Game/WallWidget.WallWidget_C"))
        (UserInterface|Viewport|AddtoViewport _returnvalue 0)
        (Input|SetInputModeGameandUI self _returnvalue "DoNotLock" true)
        (Variables|Default|SetbShowMouseCursor true)))))

(event Input|ActionEvents|InputActionDestroyWall
  (params (Key :type Key%20Structure :default "None"))
  (:Pressed
    (Actor|DestroyActor)))

(fn ConstructionScript)